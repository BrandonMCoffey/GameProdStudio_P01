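; Footstep anim notify that plays a sound based on the physical surface found by a trace.
; On notify, GetSurface runs a Visibility line trace from player character 0, not the animated mesh, to 150 units above, as the subtracted Z offset is negative.
; Concrete hits play the concrete footstep cue at the impact point and set a numeric surface code.
; Other surfaces set a default code, with no sound assigned.
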(fn ReceivedNotify
  (params (MeshComp :type Skeletal%20Mesh%20Component%20Object%20Reference) (Animation :type Anim%20Sequence%20Base%20Object%20Reference) (EventReference :type Anim%20Notify%20Event%20Reference%20Structure%20%28by%20ref%29))
  (Utilities|IsValid MeshComp
    (:Is%20Valid
      (bind _surface (CallFunction|GetSurface))
      (bind _output_get (LocalVariables|SetSurface%20Type%20Num _surface))
      (Utilities|FlowControl|Sequence
        (:then_0
          (if (== _output_get 2.0)
            (return true)))))
    (:Is%20Not%20Valid
      (return true))))

(fn GetSurface
  (bind _returnvalue (Game|GetPlayerCharacter 0))
  (bind _returnvalue_2 (Transformation|GetActorLocation _returnvalue))
  (bind (_outhit _returnvalue_3) (Collision|LineTraceByChannel _returnvalue_2 (- _returnvalue_2 "0.000000,0.000000,-150.000000") "TraceTypeQuery1" false 0 "None"))
  (if _returnvalue_3
    (switch Utilities|FlowControl|Switch|SwitchonEPhysicalSurface (Collision|GetSurfaceType _outhit)
      (:SurfaceType_Default
        (LocalVariables|SetSurface%20Type%20Num 1.0)
        (Audio|PlaySoundatLocation 0 (.Location (Collision|BreakHitResult _outhit)) "0, 0, 0" 1.0 1.0 0.0 0 0 0 0)
        (return (LocalVariables|GetSurface%20Type%20Num)))
      (:SurfaceType2
        (LocalVariables|SetSurface%20Type%20Num 2.0)
        (Audio|PlaySoundatLocation "/Game/Audio/Concrete/Concrete/SCue_Concrete_Footstep.SCue_Concrete_Footstep" (.Location (Collision|BreakHitResult _outhit)) "0, 0, 0" 1.0 1.0 0.0 0 0 0 0)))))