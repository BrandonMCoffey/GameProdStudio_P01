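; BP_Framerate is an optimization helper Blueprint that shows an on-screen FPS counter.
; ToggleFramerateDisplay creates the WB_FramerateDisplay widget and resets its counters, or removes the widget if it is already shown.
; While the widget exists, Tick counts frames and accumulates delta time, then every RefreshTime interval pushes the averaged frames per second to it.
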(event Custom|ToggleFramerateDisplay
  (bind _frameratewidget (Variables|Default|GetFrameRateWidget)
    (:then
      (Widget|RemovefromParent _frameratewidget)
      (Variables|Default|SetFrameRateWidget 0))
    (:else
      (bind _returnvalue (UserInterface|CreateWidget "/Game/Blueprints/Optimization/WB_FramerateDisplay.WB_FramerateDisplay_C"))
      (bind _output_get (Variables|Default|SetFrameRateWidget _returnvalue))
      (UserInterface|Viewport|AddtoViewport _output_get 0)
      (Variables|Default|SetRefreshTimer 0.0)
      (Variables|Default|SetRenderCount 0))))

(event EventTick
  (params (DeltaSeconds :type Float%20%28single-precision%29))
  (Variables|Default|GetFrameRateWidget
    (:then
      (bind _output_get (Variables|Default|SetRefreshTimer (+ DeltaSeconds (Variables|Default|GetRefreshTimer))))
      (if (>= _output_get (Variables|Default|GetRefreshTime))
        (Default|SetFrameRate (Variables|Default|GetFrameRateWidget) (Utilities|Text|FormatText "{fps}fps" (/ (+ (Variables|Default|GetRenderCount) 1) (Variables|Default|GetRefreshTime))))
        (Variables|Default|SetRefreshTimer 0.0)
        (Variables|Default|SetRenderCount 0)
        (else
          (Variables|Default|SetRenderCount (+ (Variables|Default|GetRenderCount) 1)))))
    (:else)))

(fn ConstructionScript)