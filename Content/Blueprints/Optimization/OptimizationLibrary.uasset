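; Blueprint function library of graphics and performance settings: High, Medium and Low quality presets, a frame rate cap and a VSync toggle.
; Each preset runs console commands that set a base Scalability level, override selected scalability groups and choose an anti-aliasing method; only High and Low set resolution quality.
; SetFrameRate builds a t.MaxFPS console command from its input, while SetVSync applies the change through GameUserSettings.
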(fn SetQualityHigh
  (Utilities|FlowControl|Sequence
    (:then_0
      (Development|ExecuteConsoleCommand 0 "Scalability 2" 0)
      (Development|ExecuteConsoleCommand 0 "sg.AntiAliasingQuality 3" 0)
      (Development|ExecuteConsoleCommand 0 "sg.ReflectionQuality 2" 0)
      (Development|ExecuteConsoleCommand 0 "sg.EffectsQuality 1" 0)
      (Development|ExecuteConsoleCommand 0 "sg.FoliageQuality 1" 0)
      (Development|ExecuteConsoleCommand 0 "sg.LandscapeQuality 1" 0)
      (Development|ExecuteConsoleCommand 0 "sg.PostProcessQuality 3" 0))
    (:then_1
      (Development|ExecuteConsoleCommand 0 "r.AntiAliasingMethod 4" 0)
      (Development|ExecuteConsoleCommand 0 "sg.ResolutionQuality 100" 0))))

(fn SetQualityMedium
  (Utilities|FlowControl|Sequence
    (:then_0
      (Development|ExecuteConsoleCommand 0 "Scalability 2" 0)
      (Development|ExecuteConsoleCommand 0 "sg.AntiAliasingQuality 1" 0)
      (Development|ExecuteConsoleCommand 0 "sg.ReflectionQuality 1" 0)
      (Development|ExecuteConsoleCommand 0 "sg.EffectsQuality 1" 0)
      (Development|ExecuteConsoleCommand 0 "sg.FoliageQuality 0" 0)
      (Development|ExecuteConsoleCommand 0 "sg.LandscapeQuality 0" 0))
    (:then_1
      (Development|ExecuteConsoleCommand 0 "r.AntiAliasingMethod 4" 0))))

(fn SetQualityLow
  (Utilities|FlowControl|Sequence
    (:then_0
      (Development|ExecuteConsoleCommand 0 "Scalability 0" 0)
      (Development|ExecuteConsoleCommand 0 "sg.AntiAliasingQuality 1" 0)
      (Development|ExecuteConsoleCommand 0 "sg.PostProcessQuality 1" 0))
    (:then_1
      (Development|ExecuteConsoleCommand 0 "r.AntiAliasingMethod 1" 0)
      (Development|ExecuteConsoleCommand 0 "sg.ResolutionQuality 50" 0))))

(fn SetFrameRate
  (params (FPS :type Integer))
  (Development|ExecuteConsoleCommand 0 (Utilities|String|Append "t.MaxFPS " (Utilities|String|ToString(Integer) FPS)) 0))

(fn SetVSync
  (params (bEnable :type Boolean))
  (bind _returnvalue (Settings|GetGameUserSettings))
  (Class|GameUserSettings|SetVSyncEnabled _returnvalue bEnable)
  (Class|GameUserSettings|ApplyNonResolutionSettings _returnvalue))