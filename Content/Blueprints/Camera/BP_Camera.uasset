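; BP_Camera is the pickup photo camera that saves shots, flips past/present switch actors and zooms, with attachable flashes and scope.
; TakePhoto runs the flash selected in WBP_CameraView, saves the SceneCapture image, then flips registered switches that are on-screen, unoccluded and match that flash.
; Sunlight and crystal flash timelines trace forward to mark actors lit, while flashless shots also trace to interact.
; Tick eases FOV zoom; SetHeld toggles physics, collision and scale.
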(event Custom|SetFov
  (params (Field%20of%20View :type Float%20%28single-precision%29))
  (Variables|/Script/Engine.SceneCaptureComponent2D|SetFOVAngle (Variables|Default|GetSceneCaptureComponent2D) Field%20of%20View)
  (Camera|SetFieldOfView (Variables|Default|GetCamera) Field%20of%20View))

(event Custom|TakePhoto
  (bind _camera (Variables|Default|GetCamera))
  (bind _returnvalue (Transformation|GetWorldLocation _camera))
  ;[0.15 0.15 0.15 0.5] No Flash Mechs
  (if (Utilities|Enum|NotEqual(Enum) (Default|GetActiveFlash (Variables|Default|GetW_CameraView)) "NewEnumerator11")
    ;[0.15 0.15 0.15 0.5] Take Photo
    (if (not (Variables|Default|GetIsTakingPhoto)) :!label _label ; Photo, Flash, and Save to Disk
      (Variables|Default|SetIsTakingPhoto true)
      (CallFunction|FlashCameraLight)
      (Utilities|FlowControl|Delay (CallFunction|GetPhotoDuration true false))
      (Default|SavePhoto (Variables|Default|GetAC_Camera) (Variables|Default|GetSceneCaptureComponent2D))
      (CallFunction|ApplyCameraEffects)
      (Audio|PlaySoundatLocation "/Game/Audio/Camera/SC_CameraTakePhoto.SC_CameraTakePhoto" (Transformation|GetActorLocation) "0, 0, 0" 1.0 1.0 0.0 0 0 0 0)
      (Utilities|FlowControl|Delay (CallFunction|GetPhotoDuration false true))
      (Variables|Default|SetIsTakingPhoto false))
    (else
      (Utilities|FlowControl|Sequence
        (:then_0
          (goto _label))
        (:then_1
          ;[0.15 0.15 0.15 0.5] Interact
          (if (Utilities|Enum|Equal(Enum) (Default|GetActiveFlash (Variables|Default|GetW_CameraView)) "NewEnumerator11") ; Interact by Camera
            (bind (_outhit _returnvalue_2) (Collision|LineTraceByChannel _returnvalue (+ _returnvalue (* (Math|Vector|GetForwardVector _camera) 5e+03)) "TraceTypeQuery3" false 0 "ForDuration"))
            (if _returnvalue_2
              (Development|PrintString (Utilities|GetDisplayName (.HitActor (Collision|BreakHitResult _outhit))))
              (if (Utilities|DoesObjectImplementInterface (.HitActor (Collision|BreakHitResult _outhit)) "/Game/Blueprints/Dialogue/BPI_Interaction.BPI_Interaction_C")
                (bind _asbp_player (Utilities|Casting|CastToBP_Player (Game|GetPlayerCharacter 0)))
                (Class|BPIInteraction|Interaction(Message) (.HitActor (Collision|BreakHitResult _outhit)) _asbp_player)))))))))

(event Custom|FlashCameraLight
  (bind _returnvalue (Transformation|GetActorLocation))
  ;[0.15 0.15 0.15 0.5] Flash Camera Light
  (switch Utilities|FlowControl|Switch|SwitchonAttachmentType (Default|GetActiveFlash (Variables|Default|GetW_CameraView))
    (:NewEnumerator9
      (Audio|PlaySoundatLocation "/Game/Audio/Camera/SC_CameraFlash.SC_CameraFlash" _returnvalue "0, 0, 0" 1.0 1.0 0.0 0 0 0 0)
      (Rendering|SetVisibility (Variables|Default|GetSpotLight) true false)
      (Rendering|Components|Light|SetLightColor (Variables|Default|GetSpotLight) "(R=1.000000,G=1.000000,B=1.000000,A=1.000000)" true)
      (Utilities|FlowControl|Sequence
        (:then_0
          (bind (_direction _flash _cone) (Timeline|SunFlashTimeline Stop)
            (:Update
              (Rendering|Components|Light|SetIntensity (Variables|Default|GetSunLight) (* _flash 8e+03))
              (Rendering|Components|Light|SetIntensity (Variables|Default|GetSpotLight) (* _flash 1.2e+03))
              (Rendering|Lighting|SetOuterConeAngle (Variables|Default|GetSpotLight) (+ (* _cone 5e+01) 1e+01)))
            (:Finished
              (Variables|Default|SetCurrentLitActor 0))
            (:TraceEvent
              (CallFunction|LineTraceSunlight))))
        (:then_1
          (bind _flash_2 (Timeline|FlashTimeline PlayFromStart)
            (:Update
              (Rendering|Components|Light|SetIntensity (Variables|Default|GetSpotLight) (* _flash_2 1.5e+02))
              (Rendering|Lighting|SetOuterConeAngle (Variables|Default|GetSpotLight) (+ (* _flash_2 3e+01) 25.0)))))))
    (:NewEnumerator1
      (Audio|PlaySoundatLocation "/Game/Audio/Camera/SC_CameraChargeSunFlash.SC_CameraChargeSunFlash" _returnvalue "0, 0, 0" 1.0 1.0 0.0 0 0 0 0 :!label _label)
      (Rendering|SetVisibility (Variables|Default|GetSpotLight) true false)
      (Rendering|Components|Light|SetLightColor (Variables|Default|GetSpotLight) "(R=1.000000,G=0.624804,B=0.303708,A=1.000000)" true)
      (Utilities|FlowControl|Sequence
        (:then_0
          (Timeline|FlashTimeline Stop))
        (:then_1
          (Timeline|SunFlashTimeline PlayFromStart))))
    (:NewEnumerator2
      (Utilities|FlowControl|Sequence
        (:then_0
          (goto _label))
        (:then_1
          (Utilities|FlowControl|DoOnce false
            (:Completed
              (bind _asbp_player (Utilities|Casting|CastToBP_Player (Game|Player|GetPlayerPawn 0)))
              (Default|QueueDialogue _asbp_player (Utilities|Struct|MakeST_DialoguePopup "" "Woah, this thing is even stronger than the sunlight bulb!" 2.0) 0.0))))))))

(event Custom|DropAndBreakSunlight
  ;[0.15 0.15 0.15 0.5] Comment
  (CallFunction|AddAttachment false "NewEnumerator1")
  (CallFunction|SetHeld false)
  (Physics|SetPhysicsLinearVelocity (Variables|Default|GetSM_Camera) "0.000000,0.000000,-100.000000" false "None")
  (Default|SwitchActiveFlash (Variables|Default|GetW_CameraView)) ; Otherwise sun flash is still selected
  (Development|PrintString "Light Broken!")
  (Utilities|FlowControl|Delay 0.25)
  (Audio|PlaySoundatLocation "/Game/Audio/Camera/SC_DropCamera.SC_DropCamera" (Transformation|GetActorLocation) "0, 0, 0" 1.0 1.0 0.0 0 0 0 0)
  (bind _returnvalue (Effects|SpawnEmitterAttached "/Game/Art/Effects/CascadeParticles/P_Sparks.P_Sparks" (Variables|Default|GetSM_Camera) "None"))
  (Utilities|FlowControl|Delay 0.3)
  (Components|Activation|SetActive _returnvalue false false))

(event Custom|SwitchActiveFlash
  (bind _selectedattachment (Default|SwitchActiveFlash (Variables|Default|GetW_CameraView)))
  (Variables|Default|SetSelectedFlash _selectedattachment))

(event Custom|SwitchActiveMode
  (params (Right :type Boolean))
  (bind _selectedattachment (Default|SwitchActiveMode (Variables|Default|GetW_CameraView) Right))
  (Variables|Default|SetSelectedMode _selectedattachment))

(event EventInteraction
  (params (Player :type BP%20Player%20Object%20Reference))
  (bind _bpc_dialogue (Variables|/Game/Blueprints/Player/BP_Player.BP_Player_C|GetBPC_Dialogue Player))
  (if (not (Variables|Default|GetHeld))
    (Default|SetCamera Player self)
    (if (not (CallFunction|HasAttachment "NewEnumerator1"))
      (Utilities|FlowControl|DoOnce false
        (:Completed
          (Default|QueueDialogue _bpc_dialogue (Utilities|Struct|MakeST_DialoguePopup "" "Yikes… the bulb is broken. There goes 40 grand of University Funding." 2.0) false)
          (Default|QueueDialogue _bpc_dialogue (Utilities|Struct|MakeST_DialoguePopup "" "Ramen’s gonna kill me… unless I get some awesome photos of this place!" 2.0) false))))))

(event EventBeginPlay
  (bind _returnvalue (UserInterface|CreateWidget "/Game/Blueprints/Camera/CameraView/WBP_CameraView.WBP_CameraView_C"))
  (bind _output_get (Variables|Default|SetW_CameraView _returnvalue))
  (UserInterface|Viewport|AddtoViewport _output_get 0)
  (Default|UpdateZoomLevel _output_get 0.0)
  (CallFunction|UpdateAttachmentVisuals)
  (Variables|Default|SetSelectedFlash (Default|GetActiveFlash (Variables|Default|GetW_CameraView))))

(event EventTick
  (params (DeltaSeconds :type Float%20%28single-precision%29))
  (Utilities|FlowControl|Sequence
    (:then_0
      (CallFunction|UpdateFov DeltaSeconds)
      (CallFunction|UpdateNotHeld))))

(fn ConstructionScript)

(fn HasAttachment
  (params (Attachment :type AttachmentType%20Enum :default "NewEnumerator0"))
  (return (Utilities|Array|ContainsItem (Variables|Default|GetAttachments) Attachment)))

(fn UpdateAttachmentVisuals
  (bind _has (CallFunction|HasAttachment "NewEnumerator1"))
  (Utilities|FlowControl|Sequence
    (:then_0
      (Default|UpdateAttachments (Variables|Default|GetW_CameraView) self))
    (:then_1
      (Rendering|SetVisibility (Variables|Default|GetLight) _has true)
      (Rendering|SetVisibility (Variables|Default|GetSpotLight) _has false)
      (Rendering|Components|Light|SetIntensity (Variables|Default|GetSpotLight) 0.0))
    (:then_2
      (Rendering|SetVisibility (Variables|Default|GetScope) (CallFunction|HasAttachment "NewEnumerator0") true))))

(fn AddAttachment
  (params (Attach :type Boolean) (Attachment :type AttachmentType%20Enum :default "NewEnumerator0"))
  (bind _attachments (Variables|Default|GetAttachments))
  (Utilities|FlowControl|Sequence
    (:then_0
      (if Attach
        (Utilities|Array|AddUnique _attachments Attachment)
        (Audio|PlaySoundatLocation "/Game/Audio/Camera/SC_CameraEquip.SC_CameraEquip" (Transformation|GetActorLocation) "0, 0, 0" 1.0 1.0 0.0 0 0 0 0)
        (else
          (Utilities|Array|RemoveItem _attachments Attachment))))
    (:then_1
      (CallFunction|UpdateAttachmentVisuals))))

(fn ToggleZoom
  (Utilities|FlowControl|Sequence
    (:then_0
      (if (>= (Variables|Default|GetZoomGoal) (Math|Float|SelectFloat 4.0 1.0 (CallFunction|HasAttachment "NewEnumerator0")))
        (Variables|Default|SetZoomGoal 0.0)
        (else
          (Variables|Default|SetZoomGoal (+ (Variables|Default|GetZoomGoal) 1.0)))))
    (:then_1
      (Default|UpdateZoomLevel (Variables|Default|GetW_CameraView) (Variables|Default|GetZoomGoal)))))

(fn ApplyCameraEffects
  (bind _returnvalue (Viewport|GetViewportSize))
  (bind _w_cameraview (Variables|Default|GetW_CameraView))
  (bind _attachmentmode (Default|GetActiveMode _w_cameraview))
  (bind _attachmentmode_2 (Default|GetActiveFlash _w_cameraview))
  (Development|PrintString "Use Camera")
  (for _array_element (Variables|Default|GetSwitches)
    (Utilities|IsValid _array_element
      (:Is%20Valid
        (if (CallFunction|CanSwitch _array_element)
          (if (and (.ReturnValue (Class|GameplayStatics|ProjectWorldtoScreen (Game|GetPlayerController 0) (+ (Transformation|GetWorldLocation (Variables|/Game/Blueprints/Switches/BP_Switch.BP_Switch_C|GetDefaultSceneRoot _array_element)) (Variables|/Game/Blueprints/Switches/BP_Switch.BP_Switch_C|GetOffsetCheck _array_element)) false)) (not (Math|Boolean|ORBoolean (< (.X (Math|Vector2D|BreakVector2D (.ScreenPosition (Class|GameplayStatics|ProjectWorldtoScreen (Game|GetPlayerController 0) (+ (Transformation|GetWorldLocation (Variables|/Game/Blueprints/Switches/BP_Switch.BP_Switch_C|GetDefaultSceneRoot _array_element)) (Variables|/Game/Blueprints/Switches/BP_Switch.BP_Switch_C|GetOffsetCheck _array_element)) false)))) 0.0) (< (.Y (Math|Vector2D|BreakVector2D (.ScreenPosition (Class|GameplayStatics|ProjectWorldtoScreen (Game|GetPlayerController 0) (+ (Transformation|GetWorldLocation (Variables|/Game/Blueprints/Switches/BP_Switch.BP_Switch_C|GetDefaultSceneRoot _array_element)) (Variables|/Game/Blueprints/Switches/BP_Switch.BP_Switch_C|GetOffsetCheck _array_element)) false)))) 0.0) (> (.X (Math|Vector2D|BreakVector2D (.ScreenPosition (Class|GameplayStatics|ProjectWorldtoScreen (Game|GetPlayerController 0) (+ (Transformation|GetWorldLocation (Variables|/Game/Blueprints/Switches/BP_Switch.BP_Switch_C|GetDefaultSceneRoot _array_element)) (Variables|/Game/Blueprints/Switches/BP_Switch.BP_Switch_C|GetOffsetCheck _array_element)) false)))) (.x _returnvalue)) (> (.Y (Math|Vector2D|BreakVector2D (.ScreenPosition (Class|GameplayStatics|ProjectWorldtoScreen (Game|GetPlayerController 0) (+ (Transformation|GetWorldLocation (Variables|/Game/Blueprints/Switches/BP_Switch.BP_Switch_C|GetDefaultSceneRoot _array_element)) (Variables|/Game/Blueprints/Switches/BP_Switch.BP_Switch_C|GetOffsetCheck _array_element)) false)))) (.y _returnvalue)))))
            (bind _returnvalue_2 (Collision|LineTraceByChannel (Transformation|GetWorldLocation (Variables|Default|GetSceneCaptureComponent2D)) (+ (Transformation|GetWorldLocation (Variables|/Game/Blueprints/Switches/BP_Switch.BP_Switch_C|GetDefaultSceneRoot _array_element)) (Variables|/Game/Blueprints/Switches/BP_Switch.BP_Switch_C|GetOffsetCheck _array_element)) "TraceTypeQuery5" true (Utilities|Array|MakeArray _array_element (Variables|/Script/Engine.ChildActorComponent|GetChildActor (Variables|/Game/Blueprints/Switches/BP_Switch.BP_Switch_C|GetPastChild _array_element)) (Variables|/Script/Engine.ChildActorComponent|GetChildActor (Variables|/Game/Blueprints/Switches/BP_Switch.BP_Switch_C|GetPresentChild _array_element))) "None"))
            (if (not _returnvalue_2)
              (Default|Switch _array_element)
              (Utilities|FlowControl|Sequence
                (:then_0
                  (if (Utilities|Array|ContainsItem (Variables|/Game/Blueprints/Switches/BP_Switch.BP_Switch_C|GetRequiredAttachments _array_element) _attachmentmode)
                    (switch Utilities|FlowControl|Switch|SwitchonAttachmentType _attachmentmode)))
                (:then_1
                  (if (Utilities|Array|ContainsItem (Variables|/Game/Blueprints/Switches/BP_Switch.BP_Switch_C|GetRequiredAttachments _array_element) _attachmentmode_2)
                    (switch Utilities|FlowControl|Switch|SwitchonAttachmentType _attachmentmode_2)))))))))))

(fn AddSwitch
  (params (NewItem :type BP%20Switch%20Object%20Reference%20%28by%20ref%29))
  (Utilities|Array|Add (Variables|Default|GetSwitches) NewItem))

(fn UpdateFov
  (params (DeltaTime :type Float%20%28double-precision%29))
  (Variables|Default|SetZoomAmount (Math|Float|Lerp (Variables|Default|GetZoomAmount) (Variables|Default|GetZoomGoal) (* DeltaTime (Variables|Default|GetZoomTransitionSpeed))))
  (CallFunction|SetFov (- 9e+01 (* (Variables|Default|GetZoomAmount) 18.75))))

(fn SetCameraActive
  (params (Active :type Boolean))
  (bind _switches (Variables|Default|GetSwitches))
  (Default|ShowUI (Variables|Default|GetW_CameraView) Active)
  (if Active
    (for _array_element _switches
      (Utilities|IsValid _array_element
        (:Is%20Valid
          (if (CallFunction|CanSwitch _array_element)
            (Default|PreviewSwitch _array_element)))))
    (else
      (for _array_element_2 _switches
        (Default|ResetPreview _array_element_2)))))

(fn CanSwitch
  (params (Switch :type BP%20Switch%20Object%20Reference))
  (for _array_element (Variables|/Game/Blueprints/Switches/BP_Switch.BP_Switch_C|GetRequiredAttachments Switch)
    (if (not (Utilities|Enum|Equal(Enum) _array_element (Default|GetActiveFlash (Variables|Default|GetW_CameraView))))
      (return false)))
  (return true))

(fn SetHeld
  (params (Held :type Boolean))
  (bind _sm_camera (Variables|Default|GetSM_Camera))
  (bind _output_get (Variables|Default|SetHeld Held))
  (Collision|SetCollisionEnabled _sm_camera (select _output_get "NoCollision" "QueryAndPhysics"))
  (Physics|SetSimulatePhysics _sm_camera (not _output_get))
  (Transformation|SetRelativeScale3D _sm_camera (Math|Vector|SelectVector "1.000000,1.000000,1.000000" "2.000000,2.000000,2.000000" _output_get))
  (Rendering|SetVisibility (Variables|Default|GetPointLight) (not _output_get) false))

(fn UpdateNotHeld
  (if (not (Variables|Default|GetHeld))
    (Transformation|SetWorldLocation (Variables|Default|GetPointLight) (+ (Transformation|GetActorLocation) "0.000000,0.000000,50.000000") false false)))

(fn LineTraceSunlight
  (bind _camera (Variables|Default|GetCamera))
  (bind _returnvalue (Transformation|GetWorldLocation _camera))
  (bind (_outhit _returnvalue_2) (Collision|LineTraceByChannel _returnvalue (+ _returnvalue (* 1e+04 (Math|Vector|GetForwardVector _camera))) "TraceTypeQuery4" false (Utilities|Array|MakeArray (Game|Player|GetPlayerPawn 0)) "ForOneFrame"))
  (if _returnvalue_2
    (if (!= (Variables|Default|GetCurrentLitActor) (.HitActor (Collision|BreakHitResult _outhit)))
      (bind _currentlitactor (Variables|Default|GetCurrentLitActor)
        (:then
          (Class|ILightReceiver|SetLit(Message) _currentlitactor false))
        (:else
          _))
      (bind _output_get (Variables|Default|SetCurrentLitActor (.HitActor (Collision|BreakHitResult _outhit))))
      (Class|ILightReceiver|SetLit(Message) _output_get true))
    (else
      (bind _currentlitactor_2 (Variables|Default|GetCurrentLitActor)
        (:then
          (Class|ILightReceiver|SetLit(Message) _currentlitactor_2 false)
          (Variables|Default|SetCurrentLitActor 0))
        (:else)))))

(fn IsFlashSunlight
  (bind _w_cameraview (Variables|Default|GetW_CameraView))
  (bind _attachmentmode (Default|GetActiveFlash _w_cameraview))
  (return (or (Utilities|Enum|Equal(Enum) _attachmentmode "NewEnumerator1") (Utilities|Enum|Equal(Enum) _attachmentmode "NewEnumerator2"))))

(fn GetPhotoDuration
  (params (Pre :type Boolean) (Post :type Boolean))
  (bind _returnvalue (CallFunction|IsFlashSunlight))
  (bind _w_cameraview (Variables|Default|GetW_CameraView))
  (bind _attachmentmode (Default|GetActiveFlash _w_cameraview))
  (bind _returnvalue_2 (Utilities|Enum|Equal(Enum) _attachmentmode "NewEnumerator11"))
  (LocalVariables|SetLocalTotal 0.0)
  (Utilities|FlowControl|Sequence
    (:then_0
      (if Pre
        (LocalVariables|SetLocalTotal (+ (LocalVariables|GetLocalTotal) (Math|Float|SelectFloat 0.05 (Math|Float|SelectFloat 1.0 0.2 _returnvalue) _returnvalue_2)))))
    (:then_1
      (if Post
        (LocalVariables|SetLocalTotal (+ (LocalVariables|GetLocalTotal) (Math|Float|SelectFloat 0.1 (Math|Float|SelectFloat 1.25 0.6 _returnvalue) _returnvalue_2)))))
    (:then_2
      (return (LocalVariables|GetLocalTotal)))))

(fn InteractText
  (return "Pickup Camera"))