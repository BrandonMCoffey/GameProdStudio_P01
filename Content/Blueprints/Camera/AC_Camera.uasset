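; Camera component that takes in-game photos and manages a gallery to view them.
; On begin play it loads or creates an SG_Photos save and prunes entries whose image files are missing from the project's Screenshots folder.
; SavePhoto captures the scene, exports the render target as a timestamped PNG and adds the file name to the save.
; ToggleGallery shows or removes WBP_Gallery, switching input mode and cursor visibility.
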(event Custom|SavePhoto
  (params (Scene%20Capture :type Scene%20Capture%20Component%202D%20Object%20Reference))
  (bind _returnvalue (Math|DateTime|Now))
  (bind _as_sg_photos (Variables|Default|GetAs%20SG%20Photos))
  (bind _returnvalue_2 (Utilities|Text|ToText(Integer) (.hour _returnvalue) false false 2))
  (bind _returnvalue_3 (Utilities|Text|ToText(Integer) (.minute _returnvalue) false false 2))
  (bind _returnvalue_4 (Utilities|Text|ToText(Integer) (.second _returnvalue) false false 2))
  (bind _returnvalue_5 (Utilities|Text|ToText(Integer) (.year _returnvalue) false false 2))
  (bind _returnvalue_6 (Utilities|Text|ToText(Integer) (.month _returnvalue) false false 2))
  (bind _returnvalue_7 (Utilities|Text|ToText(Integer) (.day _returnvalue) false false 2))
  (bind _result (Utilities|Text|FormatText " MateoLeónPhoto{DD}{MM}{YYYY}{HH}{MI}{SS}.png" _returnvalue_7 _returnvalue_6 _returnvalue_5 _returnvalue_2 _returnvalue_3 _returnvalue_4))
  (bind _returnvalue_8 (Utilities|String|ToString(Text) _result))
  ;[0 0 0 0.5] Take Photos
  ;;[0.15 0.15 0.15 0.5] Can skip this and just use the camcorder RT that is already captured
  (Rendering|SceneCapture|CaptureScene Scene%20Capture :!class /Script/Engine.SceneCaptureComponent2D)
  (bind _output_get (Variables|Default|SetPhoto (Variables|/Script/Engine.SceneCaptureComponent2D|GetTextureTarget Scene%20Capture)))
  (bind _output_get_2 (Variables|Default|SetFile%20Name _returnvalue_8))
  (Class|ImageWriteBlueprintLibrary|ExporttoDisk _output_get (Utilities|String|Append (Utilities|String|Append (Class|KismetSystemLibrary|GetProjectDirectory) "Screenshots/") _returnvalue_8) (Utilities|Struct|MakeImageWriteOptions "PNG" "(null).None"))
  (Variables|Default|SetPhoto 0)
  ;[0 0 0 0.5] Save File Name
  (Utilities|Array|Add (Variables|/Game/Blueprints/Camera/SG_Photos.SG_Photos_C|GetPhoto%20File%20Name _as_sg_photos) (Variables|Default|GetFile%20Name))
  (SaveGame|SaveGametoSlot _as_sg_photos (Variables|Default|GetSaveSlotName))
  (Development|PrintString "Updated Save Data"))

(event Custom|Toggle%20Gallery
  (bind _returnvalue (Game|GetPlayerController 0))
  (bind _returnvalue_2 (Game|GetPlayerController 0))
  ;[0 0 0 0.5] Open/Close Gallery
  (bind _gallerywidget (Variables|Default|GetGalleryWidget)
    (:then
      (Widget|RemovefromParent _gallerywidget)
      (Variables|Default|SetGalleryWidget 0)
      (Input|SetInputModeGameOnly _returnvalue false)
      (Variables|/Script/Engine.PlayerController|SetbShowMouseCursor _returnvalue false))
    (:else
      (bind _returnvalue_3 (UserInterface|CreateWidget "/Game/Blueprints/Camera/Gallery/WBP_Gallery.WBP_Gallery_C" 0 self))
      (bind _output_get (Variables|Default|SetGalleryWidget _returnvalue_3))
      (UserInterface|Viewport|AddtoViewport _output_get 0)
      (Input|SetInputModeGameandUI _returnvalue_2 _output_get "DoNotLock" true false)
      (Variables|/Script/Engine.PlayerController|SetbShowMouseCursor _returnvalue_2 true))))

(event Custom|Validate%20Save%20Data
  ;[0 0 0 0.5] Validate Save Data
  (bind _returnvalue (SaveGame|DoesSaveGameExist (Variables|Default|GetSaveSlotName)))
  (if _returnvalue
    (bind _returnvalue_2 (SaveGame|LoadGamefromSlot (Variables|Default|GetSaveSlotName)))
    (bind _assg_photos (Utilities|Casting|CastToSG_Photos _returnvalue_2))
    (Variables|Default|SetAs%20SG%20Photos _assg_photos)
    (CallFunction|DeleteInvalidPhotos)
    (else
      (bind _returnvalue_3 (SaveGame|CreateSaveGameObject "/Game/Blueprints/Camera/SG_Photos.SG_Photos_C"))
      (Variables|Default|SetAs%20SG%20Photos _returnvalue_3)))
  (SaveGame|SaveGametoSlot (Variables|Default|GetAs%20SG%20Photos) (Variables|Default|GetSaveSlotName))
  (Development|PrintString (Utilities|String|Append "Loaded " (Utilities|String|ToString(Integer) (Utilities|Array|Length (Variables|/Game/Blueprints/Camera/SG_Photos.SG_Photos_C|GetPhoto%20File%20Name (Variables|Default|GetAs%20SG%20Photos)))) " Images!")))

(event Custom|Delete%20Invalid%20Photos
  (bind _as_sg_photos (Variables|Default|GetAs%20SG%20Photos))
  (bind _photo_file_name (Variables|/Game/Blueprints/Camera/SG_Photos.SG_Photos_C|GetPhoto%20File%20Name _as_sg_photos))
  ;[0 0 0 0.5] Validate Save Data
  (bind (_arrayindex _arrayelement) (Utilities|Array|ReverseforEachLoop _photo_file_name)
    (:LoopBody
      (if (not (Class|BlueprintPathsLibrary|FileExists (Utilities|String|Append (Utilities|String|Append (Class|KismetSystemLibrary|GetProjectDirectory) "Screenshots/") _arrayelement)))
        (Development|PrintString (Utilities|String|Append "Removing Invalid Image (" (Utilities|String|Append (Utilities|String|Append (Class|KismetSystemLibrary|GetProjectDirectory) "Screenshots/") _arrayelement) ")"))
        (Utilities|Array|RemoveIndex _photo_file_name _arrayindex)))))

(event EventBeginPlay
  (CallFunction|ValidateSaveData))