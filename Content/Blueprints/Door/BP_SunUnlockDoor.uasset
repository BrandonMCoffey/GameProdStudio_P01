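; A sun symbol actor that opens a linked door when it is lit.
; On begin play it creates a dynamic material for the symbol with a near-black glow.
; When SetLit receives true, an unlocked door opens once, the player's dialogue component plays a line immediately and the symbol glows bright blue.
; A locked door is notified instead, and any linked DisableTrigger is disabled in either case.
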(event EventBeginPlay
  (bind _returnvalue (Rendering|Material|CreateDynamicMaterialInstance (Variables|Default|GetSunSymbol) 0 "/Game/Art/Symbols/MI_SymbolSun.MI_SymbolSun" "None" :!class /Script/Engine.PrimitiveComponent))
  (bind _output_get (Variables|Default|SetMaterial _returnvalue))
  (Rendering|Material|SetVectorParameterValue _output_get "Glow" "(R=0.005000,G=0.005000,B=0.005000,A=1.000000)" :!class /Script/Engine.MaterialInstanceDynamic))

(event EventSetLit
  (params (IsLit :type Boolean))
  (if IsLit
    (Utilities|FlowControl|Sequence
      (:then_0
        (bind _door (Variables|Default|GetDoor)
          (:then
            (if (Default|IsUnlocked _door)
              (Utilities|FlowControl|DoOnce false
                (:Completed
                  (Utilities|FlowControl|Sequence
                    (:then_0
                      (Default|OpenDoor (Variables|Default|GetDoor))
                      (bind _asbp_player (Utilities|Casting|CastToBP_Player (Game|Player|GetPlayerPawn 0)))
                      (Default|QueueDialogue (Variables|/Game/Blueprints/Player/BP_Player.BP_Player_C|GetBPC_Dialogue _asbp_player) (Variables|Default|GetDialogue) true))
                    (:then_1
                      (Rendering|Material|SetVectorParameterValue (Variables|Default|GetMaterial) "Glow" "(R=0.000000,G=1.232498,B=10.000000,A=1.000000)" :!class /Script/Engine.MaterialInstanceDynamic)))))
              (else
                (Default|NotifyIsLocked (Variables|Default|GetDoor)))))
          (:else)))
      (:then_1
        (bind _disabletrigger (Variables|Default|GetDisableTrigger)
          (:then
            (Default|DisableTrigger _disabletrigger))
          (:else))))))

(fn ConstructionScript)