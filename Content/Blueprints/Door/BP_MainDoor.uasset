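; Main door puzzle actor with two glyph symbols that light up as each side is solved.
; Tick polls each side's optional trigger and counts switches out of their normal state, latching that side's dynamic material glow once enough are flipped.
; A locked notification pulses unsolved glyphs and queues one-time player hint dialogue, as does the interact text query.
; IsUnlocked reports when both sides are done; the OpenDoor call here is unwired.
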(event EventBeginPlay
  (|CallParentFunction)
  (Utilities|FlowControl|Sequence
    (:then_0
      (bind _returnvalue (Rendering|Material|CreateDynamicMaterialInstance (Variables|Default|GetSymbolRight) 0 "/Game/Art/Symbols/M_Symbol_MainDoor.M_Symbol_MainDoor" "None" :!class /Script/Engine.PrimitiveComponent))
      (bind _output_get (Variables|Default|SetRightMaterial _returnvalue))
      (Rendering|Material|SetVectorParameterValue _output_get "Glow" "(R=0.000000,G=0.000000,B=0.000000,A=1.000000)" :!class /Script/Engine.MaterialInstanceDynamic))
    (:then_1
      (bind _returnvalue_2 (Rendering|Material|CreateDynamicMaterialInstance (Variables|Default|GetSymbolLeft) 0 "/Game/Art/Symbols/M_Symbol_MainDoor.M_Symbol_MainDoor" "None" :!class /Script/Engine.PrimitiveComponent))
      (bind _output_get_2 (Variables|Default|SetLeftMaterial _returnvalue_2))
      (Rendering|Material|SetVectorParameterValue _output_get_2 "Glow" "(R=0.000000,G=0.000000,B=0.000000,A=1.000000)" :!class /Script/Engine.MaterialInstanceDynamic))))

(event EventNotifyIsLocked
  (Utilities|FlowControl|Sequence
    (:then_0
      (bind _delta (Timeline|LockedNotifyTimeline PlayFromStart)
        (:Update
          (Utilities|FlowControl|Sequence
            (:then_0
              (if (not (Variables|Default|GetRightDone))
                (Rendering|Material|SetVectorParameterValue (Variables|Default|GetRightMaterial) "Glow" (Math|Color|MakeColor _delta 0.0 0.0) :!class /Script/Engine.MaterialInstanceDynamic)))
            (:then_1
              (if (not (Variables|Default|GetLeftDone))
                (Rendering|Material|SetVectorParameterValue (Variables|Default|GetLeftMaterial) "Glow" (Math|Color|MakeColor _delta 0.0 0.0) :!class /Script/Engine.MaterialInstanceDynamic)))))))
    (:then_1
      (if (or (Variables|Default|GetRightDone) (Variables|Default|GetLeftDone))
        (Utilities|FlowControl|DoOnce false
          (:Completed
            (bind _asbp_player (Utilities|Casting|CastToBP_Player (Game|Player|GetPlayerPawn 0)))
            (Default|QueueDialogue _asbp_player (Utilities|Struct|MakeST_DialoguePopup "" "Ok, taking a photo lit up the first glyph. Now I need one more." 2.0) 0.0)))
        (else
          (Utilities|FlowControl|DoOnce false
            (:Completed
              (bind _asbp_player_2 (Utilities|Casting|CastToBP_Player (Game|Player|GetPlayerPawn 0)))
              (Default|QueueDialogue _asbp_player_2 (Utilities|Struct|MakeST_DialoguePopup "" "Hmmm, the sun alone isn’t enough. Maybe there’s another mechanism?" 2.0) 0.0))))))))

(event EventTick
  (params (DeltaSeconds :type Float%20%28single-precision%29))
  (|CallParentFunction DeltaSeconds)
  (CallFunction|Check))

(fn ConstructionScript
  (bind _door (Variables|Default|GetDoor))
  (|CallParentFunction)
  (Transformation|AttachComponentToComponent (Variables|Default|GetSymbolLeft) _door "None" "KeepWorld" "KeepWorld" "KeepWorld" true)
  (Transformation|AttachComponentToComponent (Variables|Default|GetSymbolRight) _door "None" "KeepWorld" "KeepWorld" "KeepWorld" true)
  (Transformation|AttachComponentToComponent (Variables|Default|GetCube) _door "None" "KeepWorld" "KeepWorld" "KeepWorld" true))

(fn Check
  (bind _lefttrigger (Variables|Default|GetLeftTrigger))
  (bind _righttrigger (Variables|Default|GetRightTrigger))
  (if (not (Variables|Default|GetOpen))
    (Utilities|FlowControl|Sequence
      (:then_0
        (if (not (Variables|Default|GetRightDone))
          (Utilities|IsValid _righttrigger
            (:Is%20Valid
              (if (Variables|/Game/Blueprints/Switches/BP_CameraZoneTrigger.BP_CameraZoneTrigger_C|GetDone _righttrigger)
                (LocalVariables|SetCount 0 :!label _label)
                (for _array_element (Variables|Default|GetRightSideSwitches)
                  (if (not (Variables|/Game/Blueprints/Switches/BP_Switch.BP_Switch_C|GetIsNormal _array_element))
                    (Math|Integer|IncrementInt (LocalVariables|GetCount))))
                (if (>= (LocalVariables|GetCount) (Variables|Default|GetRightSideRequired))
                  (Variables|Default|SetRightDone true)
                  (Rendering|Material|SetVectorParameterValue (Variables|Default|GetRightMaterial) "Glow" "(R=0.000000,G=1.232498,B=10.000000,A=1.000000)" :!class /Script/Engine.MaterialInstanceDynamic))))
            (:Is%20Not%20Valid
              (goto _label)))))
      (:then_1
        (if (not (Variables|Default|GetLeftDone))
          (Utilities|IsValid _lefttrigger
            (:Is%20Valid
              (if (Variables|/Game/Blueprints/Switches/BP_CameraZoneTrigger.BP_CameraZoneTrigger_C|GetDone _lefttrigger)
                (LocalVariables|SetCount 0 :!label _label_2)
                (for _array_element_2 (Variables|Default|GetLeftSideSwitches)
                  (if (not (Variables|/Game/Blueprints/Switches/BP_Switch.BP_Switch_C|GetIsNormal _array_element_2))
                    (Math|Integer|IncrementInt (LocalVariables|GetCount))))
                (if (>= (LocalVariables|GetCount) (Variables|Default|GetLeftSideRequired))
                  (Variables|Default|SetLeftDone true)
                  (Rendering|Material|SetVectorParameterValue (Variables|Default|GetLeftMaterial) "Glow" "(R=0.000000,G=1.232498,B=10.000000,A=1.000000)" :!class /Script/Engine.MaterialInstanceDynamic))))
            (:Is%20Not%20Valid
              (goto _label_2))))))))

(fn IsUnlocked
  (return (and (Variables|Default|GetRightDone) (Variables|Default|GetLeftDone))))

(fn CheckDialogue
  (if (not (Variables|Default|GetDialogye))
    (bind _asbp_player (Utilities|Casting|CastToBP_Player (Game|Player|GetPlayerPawn 0)))
    (Variables|Default|SetDialogye true)
    (Default|QueueDialogue _asbp_player (Utilities|Struct|MakeST_DialoguePopup "" "Another sun-spot thingy! I’ll need more sunlight to activate it." 2.0) 0.0)))

(fn InteractText
  (CallFunction|CheckDialogue)
  (return ""))