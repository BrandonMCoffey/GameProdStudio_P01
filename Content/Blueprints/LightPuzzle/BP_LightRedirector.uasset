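; Light puzzle redirector that the player rotates in timed yaw steps to aim a light beam at ILightReceiver actors.
; While rotating, a visibility trace stretches the beam to the hit point and moves the lit message from the previous receiver to the new one.
; SetLit toggles beam visibility, and construction pre-aims it at an optional StartLookingAt actor.
; Touching the box triggers a one-time player dialogue, flagged on the game instance.
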(event OnComponentBeginOverlap(Box)
  (params (OverlappedComponent :type Primitive%20Component%20Object%20Reference) (OtherActor :type Actor%20Object%20Reference) (OtherComp :type Primitive%20Component%20Object%20Reference) (OtherBodyIndex :type Integer) (bFromSweep :type Boolean) (SweepResult :type Hit%20Result%20Structure%20%28by%20ref%29))
  (bind _asbp_player (Utilities|Casting|CastToBP_Player OtherActor))
  (bind _asbp_game_instance (Utilities|Casting|CastToBP_GameInstance (Game|GetGameInstance)))
  (if (not (Variables|/Game/Blueprints/Optimization/BP_GameInstance.BP_GameInstance_C|GetTouchLightReaction _asbp_game_instance))
    (Variables|/Game/Blueprints/Optimization/BP_GameInstance.BP_GameInstance_C|SetTouchLightReaction _asbp_game_instance true)
    (Utilities|FlowControl|DoOnce false
      (:Completed
        (Default|QueueDialogue _asbp_player (Utilities|Struct|MakeST_DialoguePopup "" "HOT!!! Is that pure sunlight? How is that possible?" 2.0) 0.0)))))

(event Custom|CamRotate)

(event EventDestroyed
  (bind _currenthit (Variables|Default|GetCurrentHit)
    (:then
      (Class|ILightReceiver|SetLit(Message) _currenthit false))
    (:else)))

(event EventSetLit
  (params (IsLit :type Boolean))
  (bind _output_get (Variables|Default|SetIsActive IsLit))
  (Rendering|SetVisibility (Variables|Default|GetLightPivot) _output_get true))

(event EventBeginPlay
  (CallFunction|TraceLine)
  (CallFunction|SetLit (Variables|Default|GetIsActive)))

(event EventInteraction
  (params (Player :type BP%20Player%20Object%20Reference))
  (Utilities|FlowControl|DoOnce false :!label _label
    (:Completed
      (Audio|PlaySoundatLocation "/Game/Audio/Puzzle/SC_PuzzleRotate.SC_PuzzleRotate" (+ (Transformation|GetActorLocation) "0.000000,0.000000,25.000000") "0, 0, 0" 1.0 1.0 0.0 0 0 0 0)
      (Components|Timeline|SetPlayRate (Variables|Default|GetRotateTimeline) (/ 1.0 (Variables|Default|GetRotateTime)))
      (Variables|Default|SetStartRotation (Variables|/Script/Engine.SceneComponent|GetRelativeRotation (Variables|Default|GetRotPivot)))
      (bind _rotatedelta (Timeline|RotateTimeline PlayFromStart)
        (:Update
          (Transformation|SetRelativeRotation (Variables|Default|GetRotPivot) (Math|Rotator|Lerp(Rotator) (Variables|Default|GetStartRotation) (Math|Rotator|CombineRotators (Variables|Default|GetStartRotation) (Math|Rotator|MakeRotator 0.0 0.0 (Variables|Default|GetRotateAmountPerInteraction))) _rotatedelta true) false false)
          (CallFunction|TraceLine))
        (:Finished
          (Utilities|FlowControl|Delay 0.2)
          (goto _label Reset))))))

(fn ConstructionScript
  (bind _lightpivot (Variables|Default|GetLightPivot))
  (bind _returnvalue (Transformation|GetWorldLocation _lightpivot))
  (Utilities|FlowControl|Sequence
    (:then_0
      (bind _startlookingat (Variables|Default|GetStartLookingAt)
        (:then
          (Transformation|SetWorldRotation (Variables|Default|GetLightPivot) (Math|Rotator|MakeRotator 0.0 0.0 (.yaw (Math|Rotator|FindLookatRotation _returnvalue (Transformation|GetActorLocation _startlookingat)))) false false)
          (Transformation|SetRelativeScale3D (Variables|Default|GetLightPivot) (Math|Vector|MakeVector 1.0 1.0 (* (Math|Vector|Distance(Vector) _returnvalue (Transformation|GetActorLocation _startlookingat)) 0.01))))
        (:else)))
    (:then_1
      (Collision|SetCollisionResponsetoChannel (Variables|Default|GetSphere) "ECC_GameTraceChannel2" (select (Variables|Default|GetCanInteract) "ECR_Block" "ECR_Ignore")))))

(fn TraceLine
  (bind _lightpivot (Variables|Default|GetLightPivot))
  (bind _returnvalue (Transformation|GetWorldLocation _lightpivot))
  (Utilities|FlowControl|Sequence
    (:then_0
      (bind (_outhit _returnvalue_2) (Collision|LineTraceByChannel _returnvalue (+ _returnvalue (* (Math|Vector|GetForwardVector _lightpivot) 1e+04)) "TraceTypeQuery1" false 0 "None"))
      (Transformation|SetRelativeScale3D (Variables|Default|GetLightPivot) (Math|Vector|MakeVector 1.0 1.0 (Math|Float|SelectFloat (* (+ (.Distance (Collision|BreakHitResult _outhit)) 5e+01) 0.01) 1e+03 _returnvalue_2)))
      (if (Utilities|DoesObjectImplementInterface (.HitActor (Collision|BreakHitResult _outhit)) "/Game/Blueprints/LightPuzzle/ILightReceiver.ILightReceiver_C")
        (LocalVariables|SetNewHit (.HitActor (Collision|BreakHitResult _outhit)))))
    (:then_1
      (bind _currenthit (Variables|Default|GetCurrentHit)
        (:then
          (if (!= _currenthit (LocalVariables|GetNewHit))
            (Class|ILightReceiver|SetLit(Message) _currenthit false)
            (bind _output_get (Variables|Default|SetCurrentHit (LocalVariables|GetNewHit) :!label _label))
            (Utilities|IsValid _output_get
              (:Is%20Valid
                (Class|ILightReceiver|SetLit(Message) _output_get true)))))
        (:else
          (goto _label))))))

(fn InteractText
  (return "Rotate"))