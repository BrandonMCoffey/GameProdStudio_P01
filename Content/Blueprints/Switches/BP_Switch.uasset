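; BP_Switch is a world object that toggles between a Present (normal) and Past (switched) state, each with a configurable mesh and child actor.
; It registers with BP_Camera on BeginPlay and offers Switch, PreviewSwitch and ResetPreview, separating actual from displayed state.
; Switch respects locking and optional one-time use, calls OnSwitch, and queues optional player dialogue the first time.
; UpdateVisuals swaps states purely through propagated component visibility.
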(event EventBeginPlay
  (CallFunction|UpdateVisuals)
  (bind _returnvalue (Actor|GetActorOfClass "/Game/Blueprints/Camera/BP_Camera.BP_Camera_C"))
  (Default|AddSwitch _returnvalue self))

(fn ConstructionScript
  (Components|StaticMesh|SetStaticMesh (Variables|Default|GetPresentSM) (Variables|Default|GetNormal_SM))
  (Components|StaticMesh|SetStaticMesh (Variables|Default|GetPastSM) (Variables|Default|GetSwitched_SM))
  (ChildActorComponent|SetChildActorClass (Variables|Default|GetPastChild) (Variables|Default|GetSwitched_BP))
  (ChildActorComponent|SetChildActorClass (Variables|Default|GetPresentChild) (Variables|Default|GetNormal_BP))
  (CallFunction|UpdateVisuals))

(fn Switch
  (if (not (Variables|Default|GetLocked))
    (if (Variables|Default|GetOneTime)
      (Variables|Default|SetLocked true))
    (bind _output_get (Variables|Default|SetIsNormal (not (Variables|Default|GetIsNormal))))
    (Variables|Default|SetIsNormal_Display _output_get)
    (Utilities|FlowControl|Sequence
      (:then_0
        (CallFunction|UpdateVisuals))
      (:then_1
        (Default|CallOnSwitch (Variables|Default|GetIsNormal)))
      (:then_2
        (Utilities|FlowControl|DoOnce false
          (:Completed
            (if (not (Utilities|Array|IsEmpty (.Dialogue (Utilities|Struct|BreakST_DialoguePopup (Variables|Default|GetDialogue)))))
              (bind _asbp_player (Utilities|Casting|CastToBP_Player (Game|Player|GetPlayerPawn 0)))
              (Default|QueueDialogue _asbp_player (Variables|Default|GetDialogue) 0.4))))))))

(fn PreviewSwitch
  (if (not (Variables|Default|GetLocked))
    (Variables|Default|SetIsNormal_Display (not (Variables|Default|GetIsNormal)))
    (CallFunction|UpdateVisuals)))

(fn ResetPreview
  (if (!= (Variables|Default|GetIsNormal) (Variables|Default|GetIsNormal_Display))
    (Variables|Default|SetIsNormal_Display (Variables|Default|GetIsNormal))
    (CallFunction|UpdateVisuals)))

(fn UpdateVisuals
  (bind _isnormal (Variables|Default|GetIsNormal))
  (bind _returnvalue (not _isnormal))
  (bind _present (Variables|Default|GetPresent)
    (:then
      (Rendering|SetVisibility _present _isnormal true))
    (:else
      _))
  (bind _past (Variables|Default|GetPast)
    (:then
      (Rendering|SetVisibility _past _returnvalue true))
    (:else
      _))
  (bind _presentchild (Variables|Default|GetPresentChild)
    (:then
      (Rendering|SetVisibility _presentchild _isnormal true))
    (:else
      _))
  (bind _pastchild (Variables|Default|GetPastChild)
    (:then
      (Rendering|SetVisibility _pastchild _returnvalue true))
    (:else)))