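; First-person player character who carries a BP_Camera actor for taking photos, switching modes and flash, and collecting attachments.
; A focus timeline raises the camera each tick between two poses, slows movement, fades its view and switches the view target, locking input during a shot.
; A per-tick line trace drives HUD prompts and BPI_Interaction calls.
; It also handles crouching, pause menu, queued dialogue and a debug note toggle.
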(event Custom|PutCameraDown
  (bind _charactermovement (Variables|Character|GetCharacterMovement))
  ;[0.15 0.15 0.15 0.5] Focus Camera
  (Variables|Default|SetInputCameraView false)
  (bind (_direction _focusdelta _camerafade _movespeedmult) (Timeline|Timeline Reverse)
    (:Update
      (Variables|Default|SetCameraFocus _focusdelta)
      (Variables|/Script/Engine.CharacterMovementComponent|SetMaxWalkSpeed _charactermovement (* (Math|Float|SelectFloat (Variables|Default|GetCrouchSpeed) (Variables|Default|GetWalkSpeed) (Variables|Default|GetIsCrouching)) _movespeedmult))
      (Variables|/Script/Engine.CharacterMovementComponent|SetMaxWalkSpeedCrouched _charactermovement (Math|Float|Clamp(Float) (Variables|Default|GetCrouchSpeed) 0.0 (* (Math|Float|SelectFloat (Variables|Default|GetCrouchSpeed) (Variables|Default|GetWalkSpeed) (Variables|Default|GetIsCrouching)) _movespeedmult)))
      (bind _camera (Variables|Default|GetCamera)
        (:then
          (Default|SetFade (Variables|/Game/Blueprints/Camera/BP_Camera.BP_Camera_C|GetW_CameraView _camera) _camerafade))
        (:else)))
    (:ShowUI
      (bind _output_get (Variables|Default|SetIsCameraFocused (and (Utilities|Select :Index _direction :Forward true :Backward false) (Utilities|IsValid (Variables|Default|GetCamera)))))
      (bind _camera_2 (Variables|Default|GetCamera)
        (:then
          (Default|SetCameraActive _camera_2 _output_get))
        (:else
          _))
      (Game|Player|SetViewTargetwithBlend (Game|GetPlayerController 0) (select (Variables|Default|GetIsCameraFocused) (Variables|Default|GetCamera) self) 0.0 "VTBlend_Linear" 0.0 false))))

(event Custom|QueueDialogue
  (params (Dialogue :type ST%20Dialogue%20Popup%20Structure) (Delay :type Float%20%28double-precision%29))
  (if (not (Utilities|Array|IsEmpty (.Dialogue (Utilities|Struct|BreakST_DialoguePopup Dialogue))))
    (if (> Delay 0.0)
      (Utilities|FlowControl|Delay Delay))
    (Default|QueueDialogue (Variables|Default|GetBPC_Dialogue) Dialogue false)))

(event Custom|TogglePauseMenu
  (bind _returnvalue (Game|GetPlayerController 0))
  (bind _returnvalue_2 (Game|GetPlayerController 0))
  (bind _w_pause (Variables|Default|GetW_Pause)
    (:then
      (Widget|RemovefromParent _w_pause)
      (Variables|Default|SetW_Pause 0)
      (Input|SetInputModeGameOnly _returnvalue true)
      (Variables|/Script/Engine.PlayerController|SetbShowMouseCursor _returnvalue false))
    (:else
      (bind _returnvalue_3 (UserInterface|CreateWidget "/Game/Blueprints/Player/W_PauseMenu.W_PauseMenu_C" 0 self))
      (bind _output_get (Variables|Default|SetW_Pause _returnvalue_3))
      (UserInterface|Viewport|AddtoViewport _output_get 0)
      (Input|SetInputModeUIOnly _returnvalue_2 _output_get "DoNotLock" false)
      (Variables|/Script/Engine.PlayerController|SetbShowMouseCursor _returnvalue_2 true))))

(event Input|EnhancedActionEvents|EnhancedInputActionIA_CameraSwitchFlash
  (params (ActionValue :type Float%20%28double-precision%29) (ElapsedSeconds :type Float%20%28double-precision%29) (TriggeredSeconds :type Float%20%28double-precision%29) (InputAction :type Input%20Action%20Object%20Reference :default "/Game/Blueprints/Player/Input/Actions/IA_CameraSwitchFlash.IA_CameraSwitchFlash"))
  ;[0.15 0.15 0.15 0.5] Camera Inputs
  (:Started
    (if (Variables|Default|GetIsCameraFocused)
      (Default|SwitchActiveFlash (Variables|Default|GetCamera)))))

(event Input|EnhancedActionEvents|EnhancedInputActionIA_Crouch
  (params (ActionValue :type Boolean) (ElapsedSeconds :type Float%20%28double-precision%29) (TriggeredSeconds :type Float%20%28double-precision%29) (InputAction :type Input%20Action%20Object%20Reference :default "/Game/Blueprints/Player/Input/Actions/IA_Crouch.IA_Crouch"))
  (bind _firstpersoncamera (Variables|Default|GetFirstPersonCamera))
  (bind _charactermovement (Variables|Character|GetCharacterMovement))
  (bind _relativelocation (Variables|/Script/Engine.SceneComponent|GetRelativeLocation _firstpersoncamera))
  (:Started
    (Variables|Default|SetIsCrouching true)
    (Variables|/Script/Engine.CharacterMovementComponent|SetMaxWalkSpeed _charactermovement 1e+02)
    (bind _alpha (Timeline|Timeline_0 Play)
      (:Update
        (Transformation|SetRelativeLocation (Variables|Default|GetFirstPersonCamera) (Math|Vector|MakeVector (.x _relativelocation) (.y _relativelocation) (Math|Float|Lerp 96.0 4e+01 _alpha)) false false)
        (Components|Capsule|SetCapsuleHalfHeight (Variables|Default|GetCapsuleComponent) (Math|Float|Lerp 96.0 4e+01 _alpha) true))))
  (:Completed
    (Variables|Default|SetIsCrouching false)
    (if (Variables|Default|GetIsCameraFocused)
      (Variables|/Script/Engine.CharacterMovementComponent|SetMaxWalkSpeed (Variables|Character|GetCharacterMovement) 1e+02)
      (else
        (Variables|/Script/Engine.CharacterMovementComponent|SetMaxWalkSpeed _charactermovement 6e+02)
        (Timeline|Timeline_0 Reverse)))))

(event Input|EnhancedActionEvents|EnhancedInputActionIA_CameraSwitchMode
  (params (ActionValue :type Float%20%28double-precision%29) (ElapsedSeconds :type Float%20%28double-precision%29) (TriggeredSeconds :type Float%20%28double-precision%29) (InputAction :type Input%20Action%20Object%20Reference :default "/Game/Blueprints/Player/Input/Actions/IA_CameraSwitchMode.IA_CameraSwitchMode"))
  (bind _camera (Variables|Default|GetCamera))
  ;[0.15 0.15 0.15 0.5] Camera Inputs
  (if (Variables|Default|GetIsCameraFocused)
    (if (> ActionValue 0.0)
      (Default|SwitchActiveMode _camera true)
      (elif (< ActionValue 0.0)
        (Default|SwitchActiveMode _camera false)))))

(event Input|EnhancedActionEvents|EnhancedInputActionIA_CameraFocus
  (params (ActionValue :type Boolean) (ElapsedSeconds :type Float%20%28double-precision%29) (TriggeredSeconds :type Float%20%28double-precision%29) (InputAction :type Input%20Action%20Object%20Reference :default "/Game/Blueprints/Player/Input/Actions/IA_CameraFocus.IA_CameraFocus"))
  (bind _charactermovement (Variables|Character|GetCharacterMovement))
  (bind _lockcamerainput (Variables|Default|GetLockCameraInput))
  ;[0.15 0.15 0.15 0.5] Focus Camera
  (:Started
    (Variables|Default|SetIsCameraFocused true)
    (Variables|Default|SetInputCameraView true)
    (if (not _lockcamerainput)
      (bind (_direction _focusdelta _camerafade _movespeedmult) (Timeline|Timeline Play)
        (:Update
          (Variables|Default|SetCameraFocus _focusdelta)
          (Variables|/Script/Engine.CharacterMovementComponent|SetMaxWalkSpeed _charactermovement (* (Math|Float|SelectFloat (Variables|Default|GetCrouchSpeed) (Variables|Default|GetWalkSpeed) (Variables|Default|GetIsCrouching)) _movespeedmult))
          (Variables|/Script/Engine.CharacterMovementComponent|SetMaxWalkSpeedCrouched _charactermovement (Math|Float|Clamp(Float) (Variables|Default|GetCrouchSpeed) 0.0 (* (Math|Float|SelectFloat (Variables|Default|GetCrouchSpeed) (Variables|Default|GetWalkSpeed) (Variables|Default|GetIsCrouching)) _movespeedmult)))
          (bind _camera (Variables|Default|GetCamera)
            (:then
              (Default|SetFade (Variables|/Game/Blueprints/Camera/BP_Camera.BP_Camera_C|GetW_CameraView _camera) _camerafade))
            (:else)))
        (:ShowUI
          (bind _output_get (Variables|Default|SetIsCameraFocused (and (Utilities|Select :Index _direction :Forward true :Backward false) (Utilities|IsValid (Variables|Default|GetCamera)))))
          (bind _camera_2 (Variables|Default|GetCamera)
            (:then
              (Default|SetCameraActive _camera_2 _output_get))
            (:else
              _))
          (Game|Player|SetViewTargetwithBlend (Game|GetPlayerController 0) (select (Variables|Default|GetIsCameraFocused) (Variables|Default|GetCamera) self) 0.0 "VTBlend_Linear" 0.0 false)))))
  (:Canceled
    (Variables|Default|SetInputCameraView false :!label _label)
    (if (not _lockcamerainput)
      (Timeline|Timeline Reverse)))
  (:Completed
    (goto _label)))

(event Input|EnhancedActionEvents|EnhancedInputActionIA_Interact
  (params (ActionValue :type Boolean) (ElapsedSeconds :type Float%20%28double-precision%29) (TriggeredSeconds :type Float%20%28double-precision%29) (InputAction :type Input%20Action%20Object%20Reference :default "/Game/Blueprints/Player/Input/Actions/IA_Interact.IA_Interact"))
  ;[0.15 0.15 0.15 0.5] Interact
  (:Started
    (CallFunction|PickupAttachmentinRange)
    (CallFunction|LineTraceInteract 8e+02 true)))

(event Input|EnhancedActionEvents|EnhancedInputActionIA_ToggleGallery
  (params (ActionValue :type Boolean) (ElapsedSeconds :type Float%20%28double-precision%29) (TriggeredSeconds :type Float%20%28double-precision%29) (InputAction :type Input%20Action%20Object%20Reference :default "/Game/Blueprints/Player/Input/Actions/IA_ToggleGallery.IA_ToggleGallery"))
  ;[0.15 0.15 0.15 0.5] Camera Inputs
  (:Started
    (Default|ToggleGallery (Variables|/Game/Blueprints/Camera/BP_Camera.BP_Camera_C|GetAC_Camera (Variables|Default|GetCamera)))))

(event Input|EnhancedActionEvents|EnhancedInputActionIA_CameraTakePhoto
  (params (ActionValue :type Boolean) (ElapsedSeconds :type Float%20%28double-precision%29) (TriggeredSeconds :type Float%20%28double-precision%29) (InputAction :type Input%20Action%20Object%20Reference :default "/Game/Blueprints/Player/Input/Actions/IA_CameraTakePhoto.IA_CameraTakePhoto"))
  (bind _camera (Variables|Default|GetCamera))
  ;[0.15 0.15 0.15 0.5] Take Photo
  (:Started
    (if (Variables|Default|GetIsCameraFocused)
      (Variables|Default|SetLockCameraInput true)
      (Default|TakePhoto _camera)
      (Default|CallOnTakePhoto)
      (Utilities|FlowControl|Delay (Default|GetPhotoDuration _camera true true))
      (Variables|Default|SetLockCameraInput false)
      (if (not (Variables|Default|GetInputCameraView))
        (CallFunction|PutCameraDown)))))

(event Input|EnhancedActionEvents|EnhancedInputActionIA_Pause
  (params (ActionValue :type Boolean) (ElapsedSeconds :type Float%20%28double-precision%29) (TriggeredSeconds :type Float%20%28double-precision%29) (InputAction :type Input%20Action%20Object%20Reference :default "/Game/Blueprints/Player/Input/Actions/IA_Pause.IA_Pause"))
  (bind _returnvalue (Game|GetPlayerController 0))
  (bind _returnvalue_2 (Game|GetPlayerController 0))
  (:Started
    (bind _w_pause (Variables|Default|GetW_Pause)
      (:then
        (Widget|RemovefromParent _w_pause)
        (Variables|Default|SetW_Pause 0)
        (Input|SetInputModeGameOnly _returnvalue true)
        (Variables|/Script/Engine.PlayerController|SetbShowMouseCursor _returnvalue false))
      (:else
        (bind _returnvalue_3 (UserInterface|CreateWidget "/Game/Blueprints/Player/W_PauseMenu.W_PauseMenu_C" 0 self))
        (bind _output_get (Variables|Default|SetW_Pause _returnvalue_3))
        (UserInterface|Viewport|AddtoViewport _output_get 0)
        (Input|SetInputModeUIOnly _returnvalue_2 _output_get "DoNotLock" false)
        (Variables|/Script/Engine.PlayerController|SetbShowMouseCursor _returnvalue_2 true)))))

(event Input|EnhancedActionEvents|EnhancedInputActionIA_CameraZoom
  (params (ActionValue :type Boolean) (ElapsedSeconds :type Float%20%28double-precision%29) (TriggeredSeconds :type Float%20%28double-precision%29) (InputAction :type Input%20Action%20Object%20Reference :default "/Game/Blueprints/Player/Input/Actions/IA_CameraZoom.IA_CameraZoom"))
  ;[0.15 0.15 0.15 0.5] Camera Inputs
  (:Started
    (Default|ToggleZoom (Variables|Default|GetCamera))))

(event EventBeginPlay
  (bind _charactermovement (Variables|Character|GetCharacterMovement))
  ;[0.15 0.15 0.15 0.5] Game Events
  (bind _returnvalue (Actor|GetActorOfClass "/Game/Blueprints/Camera/BP_Camera.BP_Camera_C"))
  (CallFunction|SetCamera _returnvalue)
  (bind _returnvalue_2 (UserInterface|CreateWidget "/Game/Blueprints/Player/W_HUD.W_HUD_C"))
  (bind _output_get (Variables|Default|SetW_HUD _returnvalue_2))
  (UserInterface|Viewport|AddtoViewport _output_get 0)
  (Variables|Default|SetWalkSpeed (Variables|/Script/Engine.CharacterMovementComponent|GetMaxWalkSpeed _charactermovement))
  (Variables|Default|SetCrouchSpeed (Variables|/Script/Engine.CharacterMovementComponent|GetMaxWalkSpeedCrouched _charactermovement))
  (CallFunction|ToggleNotesVisible))

(event EventTick
  (params (DeltaSeconds :type Float%20%28single-precision%29))
  ;[0.15 0.15 0.15 0.5] Game Events
  (|CallParentFunction DeltaSeconds)
  (CallFunction|UpdateCamera DeltaSeconds)
  (CallFunction|LineTraceInteract 8e+02 false))

(event Input|KeyboardEvents|DebugKeyN
  (params (Key :type Key%20Structure :default "None") (ActionValue :type Input%20Action%20Value%20Structure))
  (:Pressed
    (CallFunction|ToggleNotesVisible)))

(fn ConstructionScript
  (|CallParentFunction))

(fn HasAttachment
  (params (Attachment :type AttachmentType%20Enum :default "NewEnumerator0"))
  (return (Default|HasAttachment (Variables|Default|GetCamera) Attachment)))

(fn UpdateCamera
  (params (DeltaTime :type Float%20%28double-precision%29))
  (bind _camnormalpos (Variables|Default|GetCamNormalPos))
  (bind _camerafocus (Variables|Default|GetCameraFocus))
  (bind _camfocuspos (Variables|Default|GetCamFocusPos))
  (bind _returnvalue (Transformation|GetWorldTransform _camnormalpos))
  (bind _returnvalue_2 (Transformation|GetWorldTransform _camfocuspos))
  ;[0.15 0.15 0.15 0.5] Focus
  (bind _camera (Variables|Default|GetCamera)
    (:then
      (Transformation|SetActorLocationAndRotation _camera (Math|Vector|Lerp(Vector) (.location _returnvalue) (.location _returnvalue_2) _camerafocus) (Math|Rotator|Lerp(Rotator) (.rotation _returnvalue) (.rotation _returnvalue_2) (Math|Float|Clamp(Float) (* _camerafocus 2.0))) false true))
    (:else)))

(fn PickupAttachmentinRange
  (bind _attachmentpickup (Variables|Default|GetAttachmentPickup)
    (:then
      (Utilities|FlowControl|Sequence
        (:then_0
          (Default|AddAttachment (Variables|Default|GetCamera) true (Variables|/Game/Blueprints/Attachments/BP_AttachmentPickup.BP_AttachmentPickup_C|GetAttachment _attachmentpickup)))
        (:then_1
          (bind _destroyotheronpickup (Variables|/Game/Blueprints/Attachments/BP_AttachmentPickup.BP_AttachmentPickup_C|GetDestroyOtherOnPickup _attachmentpickup)
            (:then
              (Actor|DestroyActor _destroyotheronpickup))
            (:else)))
        (:then_2
          (if (Variables|/Game/Blueprints/Attachments/BP_AttachmentPickup.BP_AttachmentPickup_C|GetDestroyOnPickup _attachmentpickup)
            (Actor|DestroyActor _attachmentpickup)))))
    (:else)))

(fn InitPlayer)

(fn LineTraceInteract
  (params (Length :type Float%20%28double-precision%29) (InteractKey :type Boolean))
  (bind _firstpersoncamera (Variables|Default|GetFirstPersonCamera))
  (bind _returnvalue (Transformation|GetWorldLocation _firstpersoncamera))
  (bind (_outhit _returnvalue_2) (Collision|LineTraceByChannel _returnvalue (+ _returnvalue (* (Math|Vector|GetForwardVector _firstpersoncamera) Length 2.0)) "TraceTypeQuery3" false 0 "None"))
  (if (and _returnvalue_2 (<= (.Distance (Collision|BreakHitResult _outhit)) Length))
    (if (and (not (Variables|Default|GetIsCameraFocused)) (Utilities|DoesObjectImplementInterface (.HitActor (Collision|BreakHitResult _outhit)) "/Game/Blueprints/Dialogue/BPI_Interaction.BPI_Interaction_C"))
      (bind _action_text (Class|BPIInteraction|InteractText(Message) (.HitActor (Collision|BreakHitResult _outhit))))
      (Default|SetPromptText (Variables|Default|GetW_HUD) (Utilities|Text|FormatText "Press E to {Action}" (Utilities|String|SelectText "Interact" _action_text (Utilities|Text|TextIsEmpty _action_text))))
      (if InteractKey
        (Development|PrintString (Utilities|String|Append "Interact with: " (Utilities|GetDisplayName (.HitActor (Collision|BreakHitResult _outhit)))))
        (Class|BPIInteraction|Interaction(Message) (.HitActor (Collision|BreakHitResult _outhit)) self))
      (else
        (Default|SetPromptText (Variables|Default|GetW_HUD) :!label _label)))
    (else
      (goto _label))))

(fn ToggleNotesVisible
  (Variables|Default|SetNotesVisible (not (Variables|Default|GetNotesVisible)))
  (bind _outactors (Actor|GetAllActorsOfClass "/Game/Art/Whitebox/BP_Note.BP_Note_C"))
  (for _array_element _outactors
    (Rendering|SetVisibility (Variables|/Game/Art/Whitebox/BP_Note.BP_Note_C|GetTextRender _array_element) (Variables|Default|GetNotesVisible) false)))

(fn SetCamera
  (params (Camera :type BP%20Camera%20Object%20Reference))
  (bind _output_get (Variables|Default|SetCamera Camera))
  (Utilities|IsValid _output_get
    (:Is%20Valid
      (Default|SetHeld _output_get true)
      (Variables|Default|SetLockCameraInput false))
    (:Is%20Not%20Valid
      (Variables|Default|SetLockCameraInput true))))