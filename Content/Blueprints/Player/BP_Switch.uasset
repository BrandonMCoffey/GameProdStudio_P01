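; BP_Switch is a world actor that swaps between a present and a past version of an object.
; Construction assigns a configurable mesh and child actor class to each era, and BeginPlay registers the switch with BP_Player.
; Switch flips IsPresent, then UpdateVisuals toggles visibility of both eras and fires OnSwitch.
; With OneTime set, only the first switch updates visuals and fires the event.
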(event EventBeginPlay
  (CallFunction|UpdateVisuals false)
  (bind _returnvalue (Actor|GetActorOfClass "/Game/Blueprints/Player/BP_Player.BP_Player_C"))
  (Default|AddSwitch _returnvalue self))

(fn ConstructionScript
  (Components|StaticMesh|SetStaticMesh (Variables|Default|GetPresentSM) (Variables|Default|GetPresentObject))
  (Components|StaticMesh|SetStaticMesh (Variables|Default|GetPastSM) (Variables|Default|GetPastObject))
  (ChildActorComponent|SetChildActorClass (Variables|Default|GetPastChild) (Variables|Default|GetPastBP))
  (ChildActorComponent|SetChildActorClass (Variables|Default|GetPresentChild) (Variables|Default|GetPresentBP))
  (CallFunction|UpdateVisuals false))

(fn Switch
  (Variables|Default|SetIsPresent (not (Variables|Default|GetIsPresent)))
  (CallFunction|UpdateVisuals true))

(fn UpdateVisuals
  (params (FromPlayer :type Boolean))
  (bind _ispresent (Variables|Default|GetIsPresent))
  (bind _returnvalue (not _ispresent))
  (if (and FromPlayer (Variables|Default|GetOneTime))
    (if (not (Variables|Default|GetCompleted))
      (Variables|Default|SetCompleted true)
      (bind _present (Variables|Default|GetPresent :!label _label)
        (:then
          (Rendering|SetVisibility _present _ispresent true))
        (:else
          _))
      (bind _past (Variables|Default|GetPast)
        (:then
          (Rendering|SetVisibility _past _returnvalue true))
        (:else
          _))
      (bind _presentchild (Variables|Default|GetPresentChild)
        (:then
          (Rendering|SetVisibility _presentchild _ispresent true))
        (:else
          _))
      (bind _pastchild (Variables|Default|GetPastChild)
        (:then
          (Rendering|SetVisibility _pastchild _returnvalue true))
        (:else
          _))
      (if FromPlayer
        (Default|CallOnSwitch _ispresent)))
    (else
      (goto _label))))