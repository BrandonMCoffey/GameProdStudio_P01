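; BP_AttachmentPickup is an in-world pickup for an attachment, labelled with a prompt built from the attachment data's pickup name and an [E] key hint.
; The label refreshes in the construction script and on BeginPlay.
; Entering its sphere registers the pickup on BP_Player and queues its dialogue with no delay.
; Leaving the sphere clears the player's pickup reference, and the pickup action itself is not handled here.
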(event OnComponentBeginOverlap(Sphere)
  (params (OverlappedComponent :type Primitive%20Component%20Object%20Reference) (OtherActor :type Actor%20Object%20Reference) (OtherComp :type Primitive%20Component%20Object%20Reference) (OtherBodyIndex :type Integer) (bFromSweep :type Boolean) (SweepResult :type Hit%20Result%20Structure%20%28by%20ref%29))
  (bind _asbp_player (Utilities|Casting|CastToBP_Player OtherActor))
  (Variables|/Game/Blueprints/Player/BP_Player.BP_Player_C|SetAttachmentPickup _asbp_player self)
  (Default|QueueDialogue _asbp_player (Variables|Default|GetDialogue) 0.0))

(event OnComponentEndOverlap(Sphere)
  (params (OverlappedComponent :type Primitive%20Component%20Object%20Reference) (OtherActor :type Actor%20Object%20Reference) (OtherComp :type Primitive%20Component%20Object%20Reference) (OtherBodyIndex :type Integer))
  (bind _asbp_player (Utilities|Casting|CastToBP_Player OtherActor))
  (Variables|/Game/Blueprints/Player/BP_Player.BP_Player_C|SetAttachmentPickup _asbp_player 0))

(event EventBeginPlay
  (CallFunction|UpdateName))

(fn ConstructionScript
  (CallFunction|UpdateName))

(fn UpdateName
  (Rendering|Components|TextRender|SetText (Variables|Default|GetPickup) (Utilities|Text|ToText(String) (Utilities|String|Append "Pickup " (.PickupName (Utilities|Struct|BreakAttachmentData (CallFunction|GetAttachmentData (Variables|Default|GetAttachment)))) " [E]"))))