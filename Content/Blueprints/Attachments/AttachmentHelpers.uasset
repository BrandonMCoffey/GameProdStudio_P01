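; AttachmentHelpers is a helper Blueprint that looks up attachment data by attachment type.
; GetAttachmentData walks every row of the attachment data table and returns the first row whose Type matches the requested one.
; When no row matches, it prints a failure message naming the type and returns a default entry with an empty pickup name.
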(fn GetAttachmentData
  (params (Type :type AttachmentType%20Enum :default "NewEnumerator0"))
  (bind _outrownames (DataTable|GetDataTableRowNames "/Game/Blueprints/Attachments/AttachmentDataTable.AttachmentDataTable"))
  (for _array_element _outrownames
    (bind _returnvalue (Utilities|GetDataTableRow "/Game/Blueprints/Attachments/AttachmentDataTable.AttachmentDataTable" _array_element)
      (:then
        (if (Utilities|Enum|Equal(Enum) (.Type (Utilities|Struct|BreakAttachmentData _returnvalue)) Type)
          (return _returnvalue)))))
  (Development|PrintString 0 (Utilities|String|Append "Failed to find data for attachment for " (Utilities|String|EnumtoString Type)))
  (return (Utilities|Struct|MakeAttachmentData "NewEnumerator0")))