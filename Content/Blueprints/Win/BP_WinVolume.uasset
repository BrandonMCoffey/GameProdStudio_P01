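; BP_WinVolume is a trigger volume that ends the game when BP_Player overlaps its box.
; On overlap it immediately queues temple-locked or temple-open dialogue, chosen by IsTempleLocked.
; A parallel delayed sequence disables input and puts the camera down, then shows W_WinScreen with UI-only input after another delay.
; The win sequence runs whether or not the temple is locked.
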(event OnComponentBeginOverlap(Box)
  (params (OverlappedComponent :type Primitive%20Component%20Object%20Reference) (OtherActor :type Actor%20Object%20Reference) (OtherComp :type Primitive%20Component%20Object%20Reference) (OtherBodyIndex :type Integer) (bFromSweep :type Boolean) (SweepResult :type Hit%20Result%20Structure%20%28by%20ref%29))
  (bind _asbp_player (Utilities|Casting|CastToBP_Player OtherActor))
  (Utilities|FlowControl|Sequence
    (:then_0
      (Utilities|FlowControl|Delay 2.0)
      (Input|DisableInput _asbp_player (Game|GetPlayerController 0))
      (Default|PutCameraDown _asbp_player)
      (Utilities|FlowControl|Delay 2.0)
      (bind _returnvalue (UserInterface|CreateWidget "/Game/Blueprints/Win/W_WinScreen.W_WinScreen_C"))
      (UserInterface|Viewport|AddtoViewport _returnvalue 0)
      (Input|SetInputModeUIOnly (Game|GetPlayerController 0) _returnvalue "DoNotLock" true))
    (:then_1
      (if (Variables|Default|GetIsTempleLocked)
        (Default|QueueDialogue _asbp_player (Variables|Default|GetDialogueTempleLocked) 0.0)
        (else
          (Default|QueueDialogue _asbp_player (Variables|Default|GetDialogueTempleOpen) 0.0))))))

(fn ConstructionScript)