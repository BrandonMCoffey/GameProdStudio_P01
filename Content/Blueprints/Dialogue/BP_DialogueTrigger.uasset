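; BP_DialogueTrigger is a box trigger that queues two dialogues on the player when BP_Player enters it.
; RunDialogue fires immediately, or through a timer when TimeToTrigger is non-zero, and a DoOnce limits it to one playback.
; With Untrigger set, leaving the box cancels the pending timer.
; DisableTrigger blocks further overlaps and clears any pending timer.
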(event OnComponentBeginOverlap(Box)
  (params (OverlappedComponent :type Primitive%20Component%20Object%20Reference) (OtherActor :type Actor%20Object%20Reference) (OtherComp :type Primitive%20Component%20Object%20Reference) (OtherBodyIndex :type Integer) (bFromSweep :type Boolean) (SweepResult :type Hit%20Result%20Structure%20%28by%20ref%29))
  (bind _timetotrigger (Variables|Default|GetTimeToTrigger))
  (if (not (Variables|Default|GetDisable))
    (bind _asbp_player (Utilities|Casting|CastToBP_Player OtherActor))
    (Variables|Default|SetPlayer _asbp_player)
    (if (Variables|Default|GetUntrigger)
      _
      (else
        (Utilities|FlowControl|DoOnce false
          (:Completed
            _))))
    (if (== _timetotrigger 0.0)
      (CallFunction|RunDialogue)
      (else
        (bind _returnvalue (Utilities|Time|SetTimerbyEvent (delegate Custom|RunDialogue) _timetotrigger))
        (Variables|Default|SetTimer _returnvalue)))))

(event OnComponentEndOverlap(Box)
  (params (OverlappedComponent :type Primitive%20Component%20Object%20Reference) (OtherActor :type Actor%20Object%20Reference) (OtherComp :type Primitive%20Component%20Object%20Reference) (OtherBodyIndex :type Integer))
  (if (Variables|Default|GetUntrigger)
    (Utilities|Casting|CastToBP_Player OtherActor)
    (Utilities|Time|ClearandInvalidateTimerbyHandle (Variables|Default|GetTimer))))

(event Custom|RunDialogue
  (bind _player (Variables|Default|GetPlayer))
  (Utilities|FlowControl|DoOnce false
    (:Completed
      (Default|QueueDialogue _player (Variables|Default|GetDialogue) 0.0)
      (Default|QueueDialogue _player (Variables|Default|GetDialogue2) 0.0))))

(event Custom|DisableTrigger
  (Variables|Default|SetDisable true)
  (Utilities|Time|ClearandInvalidateTimerbyHandle (Variables|Default|GetTimer)))

(fn ConstructionScript)