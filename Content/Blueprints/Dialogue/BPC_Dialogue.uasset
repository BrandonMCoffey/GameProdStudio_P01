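; Dialogue component that shows queued dialogue lines on screen through a WBP_Dialogue typewriter widget.
; It creates the widget at BeginPlay and plays a new line at once if marked immediate or nothing is running, otherwise queues it.
; When the widget reports a line finished, it plays the next queued line or removes the widget from the viewport.
; Empty lines are not shown.
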(event Custom|QueueDialogue
  (params (Dialogue :type ST%20Dialogue%20Popup%20Structure) (Immediate :type Boolean))
  (if (or Immediate (not (Variables|Default|GetRunning)))
    (CallFunction|RunDialogue Dialogue)
    (else
      (Utilities|Array|Add (Variables|Default|GetDialogueQueue) Dialogue)
      (Development|PrintString "Queued Dialogue"))))

(event Custom|RunDialogue
  (params (Dialogue :type ST%20Dialogue%20Popup%20Structure))
  (bind _dialogue (Utilities|Struct|BreakST_DialoguePopup Dialogue))
  (Development|PrintString (Utilities|String|Append "Dialogue: " _dialogue))
  (if (> (Utilities|String|Len _dialogue) 0)
    (Variables|Default|SetRunning true)
    (Utilities|FlowControl|Sequence
      (:then_0
        (if (not (Variables|Default|GetShown))
          (UserInterface|Viewport|AddtoViewport (Variables|Default|GetWBP_DialogueRef) 0)
          (Variables|Default|SetShown true)))
      (:then_1
        (Default|ShowText (Variables|Default|GetWBP_DialogueRef) Dialogue)))))

(event Custom|OnDialogueFinished
  (bind _dialoguequeue (Variables|Default|GetDialogueQueue))
  (Variables|Default|SetRunning false)
  (if (CallFunction|AnyDialogueinQueue)
    (CallFunction|RunDialogue (Utilities|Array|Get(acopy) _dialoguequeue))
    (Utilities|Array|RemoveIndex _dialoguequeue)
    (Development|PrintString "Playing Queued Dialogue")
    (else
      (Widget|RemovefromParent (Variables|Default|GetWBP_DialogueRef))
      (Variables|Default|SetShown false)
      (Development|PrintString "Dialogue Finished"))))

(event EventBeginPlay
  (bind _returnvalue (UserInterface|CreateWidget "/Game/Blueprints/Dialogue/WBP_Dialogue.WBP_Dialogue_C"))
  (bind _output_get (Variables|Default|SetWBP_DialogueRef _returnvalue))
  (EventDispatchers|BindEventtoDialogueFinished _output_get (delegate Custom|OnDialogueFinished)))

(fn AnyDialogueinQueue
  (return (> (Utilities|Array|Length (Variables|Default|GetDialogueQueue)) 0)))